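; Physics-driven airplane actor that moves through forces on its Chassi body and is steered by the mouse.
; Helice applies constant forward thrust, mouse-driven roll and pitch torque, and offset upward lift proportional to speed.
; A separate Tick event spins the Propeller mesh a fixed step per frame, independent of delta time.
; No call to Helice appears in the file.
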(event `self.ReceiveBeginPlay`)

(event `self.ReceiveTick`
  (params (DeltaSeconds :type "Float (single-precision)"))
  (bind _returnvalue (`GameplayStatics.GetPlayerController` 0))
  (bind _chassi (`self.Chassi`))
  (bind _chassi_2 (`self.Chassi`))
  (`SceneComponent.K2_AddRelativeRotation` (`self.Propeller`) (struct :`Pitch` 42.0) false false)
  (`PrimitiveComponent.AddForceAtLocationLocal` _chassi (10000000.0 0.0 0.0) (0.0 0.0 10.0) "None")
  (`PrimitiveComponent.AddTorqueInRadians` _chassi (`KismetMathLibrary.TransformDirection` (`SceneComponent.K2_GetComponentToWorld` _chassi) (`KismetMathLibrary.MakeVector` (* (`PlayerController.GetInputAnalogKeyState` _returnvalue "MouseX") -1.0) (`PlayerController.GetInputAnalogKeyState` _returnvalue "MouseY"))) "None" true)
  (`PrimitiveComponent.AddForceAtLocationLocal` _chassi_2 (* (`KismetMathLibrary.MakeVector` 0.0 0.0 (`KismetMathLibrary.VSize` (`SceneComponent.GetComponentVelocity` _chassi_2))) 1000.0) (-70.0 0.0 0.0) "None"))

(fn `UserConstructionScript`)